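; BP_Marine is the player-controlled marine character, with movement, look, sprint and rifle firing.
; On BeginPlay it spawns a rifle, attaches it to the mesh socket and adds the W_PlayerHUD widget, passing itself in.
; Input drives capsule-relative movement, calls the weapon's Fire, and raises walk speed for sprinting when an axis value is full.
; A FlipFlop toggles third- and first-person cameras, enabling controller-yaw rotation only in first person.
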(event EventBeginPlay
  ;[0 1 0.02563] GunAppearance
  (bind _returnvalue (Game|SpawnActorfromClass "/Game/Packeges/Weapons/BP_Rifle.BP_Rifle_C" (Math|Transform|MakeTransform "0, 0, 0") "Undefined" 0 0))
  (bind _output_get (Variables|Default|SetWeapon _returnvalue))
  (Transformation|AttachComponentToComponent _output_get (Variables|Character|GetMesh) "RIfle" "KeepRelative" "KeepRelative" "KeepRelative" true)
  ;[1 1 1] WPLAYERHUD
  (bind _returnvalue_2 (UserInterface|CreateWidget "/Game/Packeges/UI/W_PlayerHUD.W_PlayerHUD_C" 0 self))
  (UserInterface|Viewport|AddtoViewport _returnvalue_2 0))

(event Input|ActionEvents|InputActionChangeCamera
  (params (Key :type Key%20Structure :default "None"))
  ;[0.09896 1 0.1756] ChangeCamera
  (:Pressed
    (Utilities|FlowControl|FlipFlop
      (:A
        (Components|Activation|Deactivate (Variables|Default|GetMainCamera%283view%29))
        (Components|Activation|Activate (Variables|Default|GetExtraCamera%281view%29) false)
        (Variables|Default|SetbUseControllerRotationYaw true))
      (:B
        (Components|Activation|Deactivate (Variables|Default|GetExtraCamera%281view%29))
        (Components|Activation|Activate (Variables|Default|GetMainCamera%283view%29) false)
        (Variables|Default|SetbUseControllerRotationYaw false)))))

(event Input|ActionEvents|InputActionSprint
  (params (Key :type Key%20Structure :default "None"))
  ;[1 0 0.01323] Sprint
  (:Pressed
    (if (== (stale Input|AxisEvents|InputAxisMoveForwardBack AxisValue) 1.0)
      (Variables|Default|Setis%20Sprinting true)
      (Variables|/Script/Engine.CharacterMovementComponent|SetMaxWalkSpeed (Variables|Character|GetCharacterMovement) 9e+02)))
  (:Released
    (Variables|Default|Setis%20Sprinting false)
    (Variables|/Script/Engine.CharacterMovementComponent|SetMaxWalkSpeed (Variables|Character|GetCharacterMovement) 6e+02)))

(event Input|ActionEvents|InputActionFire
  (params (Key :type Key%20Structure :default "None"))
  ;[1 1 1] Fire
  (:Pressed
    (Default|Fire (Variables|Default|GetWeapon))))

(event Input|AxisEvents|InputAxisMoveForwardBack
  (params (AxisValue :type Float%20%28single-precision%29))
  ;[1 1 1] Movement
  (Pawn|Input|AddMovementInput (Math|Vector|GetForwardVector (Variables|Collision|GetCapsuleComponent)) AxisValue false))

(event Input|AxisEvents|InputAxisMoveRightLeft
  (params (AxisValue :type Float%20%28single-precision%29))
  ;[1 1 1] Movement
  (Pawn|Input|AddMovementInput (Math|Vector|GetRightVector (Variables|Collision|GetCapsuleComponent)) AxisValue false))

(event Input|AxisEvents|InputAxisLookUpDown
  (params (AxisValue :type Float%20%28single-precision%29))
  ;[0.854 0.3906 1] Mouse
  (Pawn|Input|AddControllerPitchInput AxisValue))

(event Input|AxisEvents|InputAxisLookLeftRight
  (params (AxisValue :type Float%20%28single-precision%29))
  ;[0.854 0.3906 1] Mouse
  (Pawn|Input|AddControllerYawInput AxisValue))

(fn ConstructionScript)
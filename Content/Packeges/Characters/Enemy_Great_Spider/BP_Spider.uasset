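; BP_Spider is a great spider enemy that moves toward the player and can be killed by overlaps.
; On BeginPlay it links itself to its health widget, then issues an AI MoveTo toward the player.
; Any overlap plays a random hit-reaction montage, even before the other actor's type is checked.
; Only Tilegeneral actors then deduct fixed damage from Health, destroying the spider when it runs out.
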(event Collision|EventActorBeginOverlap
  (params (OtherActor :type Actor%20Object%20Reference))
  ;[1 1 1] Comment
  (Animation|Montage|PlayMontage (Variables|Character|GetMesh) (Utilities|Select :Index (Math|Random|RandomInteger 3) :Option%200 (Variables|Default|GetStunned) :Option%201 (Variables|Default|GetKnockback) :Option%202 (Variables|Default|GetHeavy))
    (:then
      (Utilities|Casting|CastToTilegeneral OtherActor)
      (Variables|Default|SetHealth (- (Variables|Default|GetHealth) 25.0))
      (if (<= (Variables|Default|GetHealth) 0.0)
        (Actor|DestroyActor)))))

(event EventBeginPlay
  ;[1 1 1] Widget login
  (bind _ashealth_widget_spider (Utilities|Casting|CastToHealth_Widget_Spider (UserInterface|GetUserWidgetObject (Variables|Default|GetHealth_Widget))))
  (Variables|/Game/Packeges/Characters/Enemy_Great_Spider/Health_Widget_Spider.Health_Widget_Spider_C|SetBP_Spider _ashealth_widget_spider self)
  (AI|AIMoveTo self "0, 0, 0" (Game|GetPlayerCharacter 0) 5.0 false))

(fn ConstructionScript)